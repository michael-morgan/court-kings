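; BP_Basketball is a basketball actor that the player character picks up by touch and can drop.
; When the player overlaps its Trigger, the Ball component stops simulating physics and colliding, then snaps to the character mesh's hand_r socket.
; It tracks possession through Looseball and AttachedActor, which GetAttachedActor exposes.
; Drop detaches a held ball, clears the holder and restores physics and collision.
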(event OnComponentBeginOverlap(Trigger)
  (params (OverlappedComponent :type Primitive%20Component%20Object%20Reference) (OtherActor :type Actor%20Object%20Reference) (OtherComp :type Primitive%20Component%20Object%20Reference) (OtherBodyIndex :type Integer) (bFromSweep :type Boolean) (SweepResult :type Hit%20Result%20Structure%20%28by%20ref%29))
  (bind _returnvalue (Game|GetPlayerCharacter 0))
  (bind _ball (Variables|Default|GetBall))
  (if (== OtherActor _returnvalue)
    (Physics|SetSimulatePhysics _ball false)
    (Collision|SetCollisionEnabled _ball "NoCollision")
    (Transformation|AttachComponentToComponent _ball (Variables|/Script/Engine.Character|GetMesh _returnvalue) "hand_r" "SnapToTarget" "KeepWorld" "KeepWorld" true)
    (Variables|Default|SetLooseball false)
    (Variables|Default|SetAttachedActor _returnvalue)))

(event EventBeginPlay)

(event Collision|EventActorBeginOverlap
  (params (OtherActor :type Actor%20Object%20Reference)))

(event EventTick
  (params (DeltaSeconds :type Float%20%28single-precision%29)))

(fn ConstructionScript)

(fn Drop
  (bind _ball (Variables|Default|GetBall))
  (if (not (Variables|Default|GetLooseball))
    (Transformation|DetachFromActor "KeepWorld" "KeepWorld" "KeepWorld")
    (Variables|Default|SetLooseball true)
    (Variables|Default|SetAttachedActor 0)
    (Physics|SetSimulatePhysics _ball true)
    (Collision|SetCollisionEnabled _ball "QueryAndPhysics")))

(fn GetAttachedActor
  (return (Variables|Default|GetAttachedActor)))